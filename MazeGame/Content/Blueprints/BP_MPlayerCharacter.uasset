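; BP_MPlayerCharacter is a player character Blueprint that produces footstep sounds and gameplay noise while moving.
; A footstep timeline starts on BeginPlay, and Tick sets its play rate from the absolute forward-movement input, so strafing alone does not drive it.
; Each timeline footstep event checks that player 0's speed is at least a small threshold, then plays the step cue and calls PawnMakeNoise at full loudness.
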(event `self.ReceiveBeginPlay`
  (`TimelineComponent.SetPlayRate` (`self.Footstep Timeline`) 0.0)
  (`Timeline|Footstep Timeline`
    (:`FootstepEvent`
      (`self.Footstep`))))

(event `self.ReceiveTick`
  (params (DeltaSeconds :type "Float (single-precision)"))
  (`TimelineComponent.SetPlayRate` (`self.Footstep Timeline`) (`KismetMathLibrary.Abs` (`self.GetInputAxisValue`))))

(fn `Footstep`
  (if (>= (`KismetMathLibrary.VSize` (`MovementComponent.Velocity` (`self.GetMovementComponent` (`GameplayStatics.GetPlayerCharacter` 0)))) 40.0)
    (`GameplayStatics.SpawnSoundAtLocation` "/Game/Audio/step_Cue.step_Cue" (`self.K2_GetActorLocation`) (struct) 1.0 1.0 0.0 null null)
    (`self.PawnMakeNoise` 1.0 (0.0 0.0 0.0) true self)))

(fn `UserConstructionScript`)